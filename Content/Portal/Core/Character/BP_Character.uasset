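; First-person character Blueprint for the Portal game, layered on a parent class that supplies the rest of its behavior.
; On BeginPlay it runs the parent logic, then flags the Mesh1P animation Blueprint as holding a rifle.
; When its capsule stops overlapping a component on a custom collision channel (GameTraceChannel5), it resets the capsule to the Pawn collision profile.
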(event `self.ReceiveBeginPlay`
  (`parent.ReceiveBeginPlay`)
  (bind _asfirst_person_anim_bp (cast `/Game/FirstPersonArms/Animations/FirstPerson_AnimBP` (`SkeletalMeshComponent.GetAnimInstance` (`self.Mesh1P`))))
  (set `/Game/FirstPersonArms/Animations/FirstPerson_AnimBP.HasRifle` true _asfirst_person_anim_bp))

(event `self.CapsuleComponent.OnComponentEndOverlap`
  (params (OverlappedComponent :type "PrimitiveComponent Object Reference") (OtherActor :type "Actor Object Reference") (OtherComp :type "PrimitiveComponent Object Reference") (OtherBodyIndex :type Integer))
  (if (`|EnumEquality` (`PrimitiveComponent.GetCollisionObjectType` OtherComp) "ECC_GameTraceChannel5")
    (`PrimitiveComponent.SetCollisionProfileName` (`self.CapsuleComponent`) "Pawn" true)))

(fn `UserConstructionScript`)