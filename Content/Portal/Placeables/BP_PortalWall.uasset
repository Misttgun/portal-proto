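; BP_PortalWall is a portal-system wall placeable whose one working function, Toto, measures a portal ghost border's footprint on the wall.
; Toto spawns a BP_GhostBorder at the given transform and converts its mesh vertices into the wall's local space.
; It returns half-width and half-height from the Y/Z bounds, drawing debug points and a box.
; The spawned border is never destroyed, and the construction script is empty.
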(fn `Toto`
  (params (Origin :type "Vector Structure") (Rotation :type "Rotator Structure"))
  (returns (Width :type "Float (double-precision)") (Height :type "Float (double-precision)"))
  (locals (MinZ :type "Float (double-precision)") (MinY :type "Float (double-precision)") (MaxZ :type "Float (double-precision)") (MaxY :type "Float (double-precision)") (LocalVertexPos :type "Vector Structure"))
  (bind (_localvertexpos_x _localvertexpos_y _localvertexpos_z) (`KismetMathLibrary.BreakVector` (`local.LocalVertexPos`)))
  (bind _returnvalue (/ (- (`local.MaxY`) (`local.MinY`)) 2.0))
  (bind _returnvalue_2 (/ (- (`local.MaxZ`) (`local.MinZ`)) 2.0))
  (bind _output_get (set `local.MinZ` 1000000.0))
  (set `local.MinY` _output_get)
  (bind _output_get_2 (set `local.MaxZ` -1000000.0))
  (set `local.MaxY` _output_get_2)
  (bind _returnvalue_3 (`|SpawnActorFromClass` "/Game/Portal/Placeables/BP_GhostBorder.BP_GhostBorder_C" (`KismetMathLibrary.MakeTransform` (`local.Origin`) (`local.Rotation`)) "AlwaysSpawn" "MultiplyWithRoot" null null))
  (bind _meshcomp (`PGhostPortalBorder.MeshComp` _returnvalue_3))
  (bind _vertices (`KismetProceduralMeshLibrary.GetSectionFromStaticMesh` (`StaticMeshComponent.StaticMesh` _meshcomp)))
  (for _array_element _vertices
    (set `local.LocalVertexPos` (`KismetMathLibrary.InverseTransformLocation` (`self.GetTransform`) (`KismetMathLibrary.TransformLocation` (`self.GetTransform` _returnvalue_3) (`KismetMathLibrary.GreaterGreater_VectorRotator` _array_element (`SceneComponent.RelativeRotation` _meshcomp)))))
    (`KismetSystemLibrary.DrawDebugPoint` (`KismetMathLibrary.TransformLocation` (`self.GetTransform`) (`local.LocalVertexPos`)) 10.0 (struct :`A` 1.0) 5.0)
    (set `local.MinY` (`KismetMathLibrary.FMin` _localvertexpos_y (`local.MinY`)))
    (set `local.MinZ` (`KismetMathLibrary.FMin` _localvertexpos_z (`local.MinZ`)))
    (set `local.MaxY` (`KismetMathLibrary.FMax` _localvertexpos_y (`local.MaxY`)))
    (set `local.MaxZ` (`KismetMathLibrary.FMax` _localvertexpos_z (`local.MaxZ`))))
  (`KismetSystemLibrary.DrawDebugBox` (`local.Origin`) (`KismetMathLibrary.MakeVector` 2.0 _returnvalue _returnvalue_2) (struct :`R` 1.0 :`G` 0.001466 :`B` 0.336579 :`A` 1.0) (`self.K2_GetActorRotation`) 10.0 1.0)
  (return _returnvalue _returnvalue_2))

(fn `UserConstructionScript`)